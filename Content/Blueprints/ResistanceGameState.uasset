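; Game state for the Resistance mode, running enemy waves round by round on the dedicated server.
; The RoundStarted rep-notify announces the round, activates Generator ambience and respawns each AISpawner with a per-round count, fixed from round three on.
; A looping timer, begun by StartTimer, polls for living first-team characters.
; When none remain, it switches Generator effects, deactivates the Resistance panel, pauses polling and advances the round.
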(event `RoundEnd`
  (bind _outactors (`GameplayStatics.GetAllActorsOfClass` "/Game/ThirdPersonBP/Blueprints/Generator.Generator_C"))
  (bind _output (`|GetArrayItem` _outactors))
  (`ActorComponent.Deactivate` (`/Game/ThirdPersonBP/Blueprints/Generator.Ambient` _output))
  (`ActorComponent.Deactivate` (`/Game/ThirdPersonBP/Blueprints/Generator.Ambient2` _output))
  (`ActorComponent.Deactivate` (`/Game/ThirdPersonBP/Blueprints/Generator.Ambient3` _output))
  (`ActorComponent.Activate` (`/Game/ThirdPersonBP/Blueprints/Generator.RIP` _output) true)
  (bind _outactors_2 (`GameplayStatics.GetAllActorsOfClass` "/Game/Items/Resistance_Panel.Resistance_Panel_C"))
  (`/Game/Items/Resistance_Panel.Deactivate` (`|GetArrayItem` _outactors_2)))

(event `RoundAnnounce`
  (bind _aswwplayer_controller (cast `/Game/ThirdPersonBP/WWPlayerController` (`GameplayStatics.GetPlayerController` 0)))
  (`/Game/ThirdPersonBP/WWPlayerController.ShowRoundAnnouncement` _aswwplayer_controller)
  (bind _outactors (`GameplayStatics.GetAllActorsOfClass` "/Game/ThirdPersonBP/Blueprints/Generator.Generator_C"))
  (bind _output (`|GetArrayItem` _outactors))
  (`ActorComponent.Activate` (`/Game/ThirdPersonBP/Blueprints/Generator.Ambient` _output) true)
  (`ActorComponent.Activate` (`/Game/ThirdPersonBP/Blueprints/Generator.Ambient2` _output) true)
  (`ActorComponent.Activate` (`/Game/ThirdPersonBP/Blueprints/Generator.Ambient3` _output) true))

(event `self.ReceiveBeginPlay`)

(event `StartTimer`
  (if (`KismetSystemLibrary.IsDedicatedServer`)
    (bind _returnvalue (`KismetSystemLibrary.K2_SetTimer` null "CheckEnemiesAlive" 3.0 true))
    (set `self.Timer` _returnvalue)))

(event `End Timer`
  (`KismetSystemLibrary.K2_PauseTimerHandle` (`self.Timer`))
  (set `self.RoundStarted` false))

(fn `CheckEnemiesAlive`
  (bind _outactors (`GameplayStatics.GetAllActorsOfClass` "/Game/ThirdPersonBP/Blueprints/ThirdPersonCharacter.ThirdPersonCharacter_C"))
  (for _array_element _outactors
    (if (`/Game/ThirdPersonBP/Blueprints/ThirdPersonCharacter.Dead` _array_element)
      _
      (elif (`|EnumEquality` (`/Game/ThirdPersonBP/Blueprints/ThirdPersonCharacter.Team` _array_element) "NewEnumerator0")
        (return))))
  (`KismetSystemLibrary.PrintString` "Do Something")
  (`self.RoundEnd`)
  (`self.End Timer`)
  (set `self.CurrentRound` (+ (`self.CurrentRound`) 1)))

(fn `OnNewRound`
  (if (`KismetSystemLibrary.IsDedicatedServer`)
    (if (`self.RoundStarted`)
      (`self.RoundAnnounce`)
      (bind _outactors (`GameplayStatics.GetAllActorsOfClass` "/Game/AISpawner.AISpawner_C"))
      (for _array_element _outactors
        (`/Game/AISpawner.respawn` _array_element (`|GetArrayItem` (`self.enemiesPerRound`) (- (`self.CurrentRound`) 1))))
      (else
        (`self.RoundEnd`)))))

(fn `OnRep_RoundStarted`
  (bind _currentround (`self.CurrentRound`))
  (if (`KismetSystemLibrary.IsDedicatedServer`)
    (if (`self.RoundStarted`)
      (`self.RoundAnnounce`)
      (bind _outactors (`GameplayStatics.GetAllActorsOfClass` "/Game/AISpawner.AISpawner_C"))
      (for _array_element _outactors
        (if (>= _currentround 3)
          (`/Game/AISpawner.respawn` _array_element 12)
          (else
            (`/Game/AISpawner.respawn` _array_element (`|GetArrayItem` (`self.enemiesPerRound`) (- _currentround 1))))))
      (else
        (`self.RoundEnd`)
        (if (> (`self.CurrentRound`) (`KismetArrayLibrary.Array_Length` (`self.enemiesPerRound`)))
          (`self.RoundEnd`))))))

(fn `UserConstructionScript`)