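; Game mode for a dedicated server that publishes the current player count in the online session's extra settings.
; On each post-login and logout, it writes the GameState PlayerArray length to the "P" session property and updates the session, preserving its other options.
; The count drops by one when the first PlayerState lacks a valid unique net ID.
; An unconnected alternative that counts PlayerController actors remains in the graph.
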(event `K2_PostLogin_1`
  (params (NewPlayer :type "PlayerController Object Reference"))
  (bind _output (`|GetArrayItem` (`GameStateBase.PlayerArray` (`GameplayStatics.GetGameState`))))
  (`/Engine/EditorBlueprintResources/StandardMacros.IsValid` _output :!label _label
    (:`Is Valid`
      (bind (_numconnections _numprivateconnections _bislan _bisdedicated _ballowinvites _ballowjoininprogress _bisanticheatenabled _builduniqueid _extrasettings) (`AdvancedSessionsLibrary.GetSessionSettings`)
        (:`OnSuccess`
          (bind _modifiedsettingsarray (`AdvancedSessionsLibrary.AddOrModifyExtraSettings` _extrasettings (`|MakeArray` (`AdvancedSessionsLibrary.MakeLiteralSessionPropertyInt` "P" (`KismetMathLibrary.SelectInt` (`KismetArrayLibrary.Array_Length` (`GameStateBase.PlayerArray` (`GameplayStatics.GetGameState`))) (- (`KismetArrayLibrary.Array_Length` (`GameStateBase.PlayerArray` (`GameplayStatics.GetGameState`))) 1) (`AdvancedSessionsLibrary.IsValidUniqueNetID` (`AdvancedSessionsLibrary.GetUniqueNetIDFromPlayerState` _output)))))))
          (`UpdateSessionCallbackProxyAdvanced.UpdateSession` _modifiedsettingsarray 100 0 _bislan _ballowinvites _ballowjoininprogress true _bisdedicated
            (:`OnSuccess`
              (`KismetSystemLibrary.PrintString` "Session Updated Successfully"))
            (:`OnFailure`
              (`KismetSystemLibrary.PrintString` "Session Failed To Update"))))))))

(event `K2_OnLogout_1`
  (params (ExitingController :type "Controller Object Reference"))
  (goto _label))

(fn `UserConstructionScript`)